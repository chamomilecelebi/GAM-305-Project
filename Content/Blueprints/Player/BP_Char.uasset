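; Side-scrolling Paper2D player character with Enhanced Input for movement along world X and jumping.
; BeginPlay adds the mapping context, then has BP_PlayerCont apply speed, jump, health and healing; a Speed event sets walk speed and a derived RotationSpeed.
; Tick turns the controller to face horizontal velocity and picks idle, run or jump flipbooks from movement state, debug-printing health while grounded.
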(event `self.ReceiveBeginPlay`
  ; Setup Player Inputs
  (bind _asplayer_controller (cast `PlayerController` (`self.GetController`)))
  (`EnhancedInputSubsystemInterface.AddMappingContext` (pcsubsystem `EnhancedInputLocalPlayerSubsystem` _asplayer_controller) "/Game/Input/IMC_SideScroller.IMC_SideScroller" 0 (struct))
  ; Player applies
  (bind _asbp_player_cont (cast `/Game/Blueprints/Player/BP_PlayerCont` (`GameplayStatics.GetPlayerController` 0)))
  (`/Game/Blueprints/Player/BP_PlayerCont.ApplySpeed` _asbp_player_cont)
  (`/Game/Blueprints/Player/BP_PlayerCont.applyJump` _asbp_player_cont)
  (`/Game/Blueprints/Player/BP_PlayerCont.applyHealth` _asbp_player_cont)
  (`/Game/Blueprints/Player/BP_PlayerCont.applyHealing` _asbp_player_cont))

(event `EnhancedInput|/Game/Input/Actions/IA_Move`
  (params (ActionValue :type "Float (double-precision)") (ElapsedSeconds :type "Float (double-precision)") (TriggeredSeconds :type "Float (double-precision)") (InputAction :type "InputAction Object Reference" :default "/Game/Input/Actions/IA_Move.IA_Move"))
  ; Player X-Axis Movement
  (:`Triggered`
    (`self.AddMovementInput` (1.0 0.0 0.0) ActionValue)))

(event `EnhancedInput|/Game/Input/Actions/IA_Jump`
  (params (ActionValue :type Boolean) (ElapsedSeconds :type "Float (double-precision)") (TriggeredSeconds :type "Float (double-precision)") (InputAction :type "InputAction Object Reference" :default "/Game/Input/Actions/IA_Jump.IA_Jump"))
  ; Player Jump Input
  (:`Triggered`
    (if ActionValue
      (`self.Jump`)
      (else
        (`self.StopJumping`)))))

(event `self.ReceiveTick`
  (params (DeltaSeconds :type "Float (single-precision)"))
  ; Update Run or Walk Sprite
  (`self.SetCharRotation`)
  (if (`NavMovementComponent.IsMovingOnGround` (`self.CharacterMovement`))
    (if (<= (`KismetMathLibrary.Abs` (`KismetMathLibrary.VSize` (`self.GetVelocity`))) 0.0)
      (`PaperFlipbookComponent.SetFlipbook` (`self.Sprite`) "/Game/Sprites/Player/S_Player_Idle.S_Player_Idle")
      (`KismetSystemLibrary.PrintString` (`KismetStringLibrary.Conv_DoubleToString` (`self.Current Health`)))
      (else
        (`PaperFlipbookComponent.SetFlipbook` (`self.Sprite`) "/Game/Sprites/Player/S_Player_Run.S_Player_Run")
        (`KismetSystemLibrary.PrintString` (`KismetStringLibrary.Conv_DoubleToString` (`self.Current Health`)))))
    (else
      (`self.SetCharJumping`))))

(event `SetCharRotation`
  (bind _returnvalue (`self.GetController`))
  (bind _returnvalue_2 (`self.GetController`))
  (bind _velocity_x (`KismetMathLibrary.BreakVector` (`MovementComponent.Velocity` (`self.GetMovementComponent`))))
  ; Sprite Rotation
  (`/Engine/EditorBlueprintResources/StandardMacros.CompareFloat` _velocity_x
    (:`>`
      (`/Engine/EditorBlueprintResources/StandardMacros.IsValid` _returnvalue_2
        (:`Is Valid`
          (`Controller.SetControlRotation` _returnvalue_2 (`KismetMathLibrary.MakeRotator` 0.0)))))
    (:`<`
      (`/Engine/EditorBlueprintResources/StandardMacros.IsValid` _returnvalue
        (:`Is Valid`
          (`Controller.SetControlRotation` _returnvalue (`KismetMathLibrary.MakeRotator` 0.0 0.0 180.0)))))))

(event `SetCharJumping`
  (bind (_velocity_x _velocity_y _velocity_z) (`KismetMathLibrary.BreakVector` (`MovementComponent.Velocity` (`self.GetMovementComponent`))))
  ; Player Jump Sprite
  (`/Engine/EditorBlueprintResources/StandardMacros.CompareFloat` _velocity_z
    (:`>`
      (`PaperFlipbookComponent.SetFlipbook` (`self.Sprite`) "/Game/Sprites/Player/S_Player_JumpStart.S_Player_JumpStart"))
    (:`<`
      (`PaperFlipbookComponent.SetFlipbook` (`self.Sprite`) "/Game/Sprites/Player/S_Player_JumpLoop.S_Player_JumpLoop"))))

(event `Speed`
  (params (Speed :type "Float (double-precision)"))
  (set `CharacterMovementComponent.MaxWalkSpeed` Speed (`self.CharacterMovement`))
  (set `self.Rotation Speed` (* Speed -0.2)))

(fn `UserConstructionScript`)