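; BP_EnemyAI is an enemy pawn that roams randomly, chases the player once seen and deals contact damage.
; It starts roaming to random reachable points on BeginPlay; PawnSensing sight switches it to AIMoveTo the player, resuming roaming only if that move fails.
; Overlapping its collider damages a BP_Char unless invincible.
; Incoming damage reduces Health and destroys the actor at zero.
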(event `self.ReceiveAnyDamage`
  (params (Damage :type "Float (single-precision)") (DamageType :type "DamageType Object Reference") (InstigatedBy :type "Controller Object Reference") (DamageCauser :type "Actor Object Reference"))
  ; Enemy Health
  (set `self.Health` (- (`self.Health`) Damage))
  (if (<= (`self.Health`) 0.0)
    (`self.K2_DestroyActor`)))

(event `self.Enemy collider.OnComponentBeginOverlap`
  (params (OverlappedComponent :type "PrimitiveComponent Object Reference") (OtherActor :type "Actor Object Reference") (OtherComp :type "PrimitiveComponent Object Reference") (OtherBodyIndex :type Integer) (bFromSweep :type Boolean) (SweepResult :type "HitResult Structure (by ref)"))
  ; enemy damage player
  (bind _asbp_char (cast `/Game/Blueprints/Player/BP_Char` OtherActor))
  (if (not (`/Game/Blueprints/Player/BP_Char.IsInvincible` _asbp_char))
    (`GameplayStatics.ApplyDamage` _asbp_char (`self.Base Damage`))))

(event `self.PawnSensing.OnSeePawn`
  (params (Pawn :type "Pawn Object Reference"))
  ; AI Move towards player
  (set `self.IsSeeingPlayer` true)
  (`self.FollowPlayer`))

(event `FollowPlayer`
  ; AI Move towards player
  (if (`self.IsSeeingPlayer`)
    (`|AIMoveTo` self (0.0 0.0 0.0) (`GameplayStatics.GetPlayerCharacter` 0)
      (:`OnFail`
        (`self.Random Roam`)))))

(event `Random Roam`
  ; AI Random Roam
  (`|AIMoveTo` self (`NavigationSystemV1.K2_GetRandomReachablePointInRadius` (`self.K2_GetActorLocation`) 5000.0 null null) null 0.25 true
    (:`OnSuccess`
      (`self.Random Roam`))
    (:`OnFail`
      (`self.Random Roam`))))

(event `self.ReceiveBeginPlay`
  ; AI Random Roam
  (`self.Random Roam`))

(fn `UserConstructionScript`)